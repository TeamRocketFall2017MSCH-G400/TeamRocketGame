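; Debris trigger actor that appears intended to release physics debris on overlap, but is unfinished.
; Its overlap event casts the other actor to PlayerController, then loops over DebrisArray with an empty body.
; Nodes that number each piece, store the total and activate the first piece are disconnected.
; The ActivateDerbris function enables physics simulation on a piece's static mesh, but no live path calls it.
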(event `self.ReceiveActorBeginOverlap`
  (params (OtherActor :type "Actor Object Reference"))
  (cast `PlayerController` OtherActor)
  (for (_array_element _array_index) (`self.DebrisArray`)
    _))

(fn `ActivateDerbris`
  (params (NextDebris :type "/Game/Blueprints/derbris Object Reference"))
  (`PrimitiveComponent.SetSimulatePhysics` (`/Game/Blueprints/derbris.StaticMesh` NextDebris) true))

(fn `UserConstructionScript`)